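; Base zombie character that spawns as a random fast, medium or slow variant and voices attack or chase sounds around tanks.
; BeginPlay rolls the variant and sound interval, then SetupZombie sets walk speed, animation class, attack sound and initial sound.
; Tick line-traces from the arrow component for a Tank_BP to choose the sound, replayed on a frame countdown via TankGameInstance's SoundManager.
; PlaySoundAtR's play call is unwired.
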(event `self.ReceiveTick`
  (params (DeltaSeconds :type "Float (single-precision)"))
  (bind _soundtimer (`self.SoundTimer`))
  (bind _arrowcomponent (`self.ArrowComponent`))
  (bind _returnvalue (`SceneComponent.K2_GetComponentLocation` _arrowcomponent))
  ;[1 1 1] Line Trace For Hit Detection
  (bind _outhit (`KismetSystemLibrary.LineTraceSingle` _returnvalue (+ _returnvalue (* (`KismetMathLibrary.GetForwardVector` (`SceneComponent.K2_GetComponentRotation` _arrowcomponent)) (`self.DistanceToHitTank`))) "TraceTypeQuery1"))
  (bind _output_get (set `self.InRangeOfTank` (`KismetMathLibrary.ClassIsChildOf` (`GameplayStatics.GetObjectClass` (`.HitActor` (`GameplayStatics.BreakHitResult` _outhit))) "/Game/Tank/Tank_BP.Tank_BP_C")))
  ;[1 1 1] Audio Management
  (if _output_get
    (set `self.CurrentSound` (`self.AttackSound`))
    (else
      (set `self.CurrentSound` (`self.ChaseSound`))))
  (if (> _soundtimer 0)
    (set `self.SoundTimer` (- _soundtimer 1))
    (else
      (`self.PlaySoundAt` (`self.CurrentSound`) 0.15 1.0 0.0 "/Game/Zombie/ZombieSoundAttenuation_BP.ZombieSoundAttenuation_BP" "/Game/Zombie/ZombieSoundConcurrency_BP.ZombieSoundConcurrency_BP")
      (set `self.SoundTimer` (`self.SoundWait`)))))

(event `self.ReceiveBeginPlay`
  ;[1 1 1] Randomly creates different type of szombie
  (set `self.SoundWait` (`KismetMathLibrary.RandomIntegerInRange` 200 400))
  (switch `int` (`KismetMathLibrary.RandomInteger` 3)
    (:`0`
      (`self.SetupZombie` (`KismetMathLibrary.Conv_IntToDouble` (`KismetMathLibrary.RandomIntegerInRange` 600 800)) "FastAttackCue" "FastChaseCue" "/Game/Zombie/FastZombieAnimation_BP.FastZombieAnimation_BP_C"))
    (:`1`
      (`self.SetupZombie` (`KismetMathLibrary.Conv_IntToDouble` (`KismetMathLibrary.RandomIntegerInRange` 400 600)) "SlowAndMediumAttackCue" "MediumChase" "/Game/Zombie/MediumZombieAnimation_BP.MediumZombieAnimation_BP_C"))
    (:`2`
      (`self.SetupZombie` (`KismetMathLibrary.Conv_IntToDouble` (`KismetMathLibrary.RandomIntegerInRange` 200 400)) "SlowAndMediumAttackCue" "SlowChaseCue" "/Game/Zombie/SlowZombieAnimation_BP.SlowZombieAnimation_BP_C"))))

(fn `PlaySoundAt`
  (params (SoundName :type String) (Volume :type "Float (double-precision)" :default 1.0) (Pitch :type "Float (double-precision)" :default 1.0) (StartTime :type "Float (double-precision)") (AttenuationSettings :type "SoundAttenuation Object Reference") (ConcurrencySettings :type "SoundConcurrency Object Reference"))
  (bind _astank_game_instance (cast `TankGameInstance` (`GameplayStatics.GetGameInstance`))
    (:`then`
      (`SoundManager.PlaySoundAt` (`TankGameInstance.SoundManager` _astank_game_instance) SoundName self (`self.K2_GetActorLocation` self) Volume Pitch StartTime AttenuationSettings ConcurrencySettings))
    (:`CastFailed`
      _))
  (return))

(fn `PlaySoundAtR`
  (params (SoundName :type String) (Volume :type "Float (double-precision)" :default 1.0) (Pitch :type "Float (double-precision)" :default 1.0) (StartTime :type "Float (double-precision)") (AttenuationSettings :type "SoundAttenuation Object Reference") (ConcurrencySettings :type "SoundConcurrency Object Reference"))
  (bind _astank_game_instance (cast `TankGameInstance` (`GameplayStatics.GetGameInstance`))
    (:`CastFailed`
      (return))))

(fn `SetupZombie`
  (params (MaxSpeed :type "Float (double-precision)") (AttackSound :type String) (ChaseSound :type String) (Animation :type "Object Class Reference"))
  (set `CharacterMovementComponent.MaxWalkSpeed` MaxSpeed (`self.CharacterMovement`))
  (set `self.AttackSound` AttackSound)
  (set `self.CurrentSound` ChaseSound)
  (`SkeletalMeshComponent.SetAnimInstanceClass` (`self.Mesh`) Animation)
  (return))

(fn `UserConstructionScript`)