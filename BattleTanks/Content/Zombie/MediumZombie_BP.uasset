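; Medium zombie Blueprint that detects when a tank is within hit range in front of it.
; Every Tick it line traces on the Visibility channel from its ArrowComponent along the arrow's forward vector for DistanceToHitTank.
; InRangeOfTank is set by whether the hit actor's class derives from Tank_BP.
; The file only updates this flag, with no attack or movement logic.
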(event `self.ReceiveTick`
  (params (DeltaSeconds :type "Float (single-precision)"))
  (bind _arrowcomponent (`self.ArrowComponent`))
  (bind _returnvalue (`SceneComponent.K2_GetComponentLocation` _arrowcomponent))
  ;[1 1 1] Line Trace For Hit Detection
  (bind _outhit (`KismetSystemLibrary.LineTraceSingle` _returnvalue (+ _returnvalue (* (`KismetMathLibrary.GetForwardVector` (`SceneComponent.K2_GetComponentRotation` _arrowcomponent)) (`self.DistanceToHitTank`))) "TraceTypeQuery1"))
  (set `self.InRangeOfTank` (`KismetMathLibrary.ClassIsChildOf` (`GameplayStatics.GetObjectClass` (`.HitActor` (`GameplayStatics.BreakHitResult` _outhit))) "/Game/Tank/Tank_BP.Tank_BP_C")))

(event `self.ReceiveBeginPlay`)

(fn `UserConstructionScript`)